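; Player character Blueprint that sets up the stamina HUD and the starting katana weapon.
; On BeginPlay it adds the stamina widget to the viewport, then spawns a katana owned by the character, tags it as a weapon and snaps it to the right-hand weapon socket on the mesh.
; Pressing R opens the VelkariiPlayground level through a hard-wired key event.
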(event `self.ReceiveBeginPlay`
  (bind _returnvalue (`|CreateWidget` "/Game/Widgets/BPW_Stamina.BPW_Stamina_C" (`GameplayStatics.GetPlayerController` 0)))
  (`UserWidget.AddToViewport` _returnvalue 0)
  (bind _returnvalue_2 (`|SpawnActorFromClass` "/Game/Weapons/Katana/Blueprints/BP_Katana.BP_Katana_C" (`KismetMathLibrary.MakeTransform` (0.0 0.0 0.0)) "Undefined" "MultiplyWithRoot" self null))
  (set `Actor.Tags` (`|MakeArray` "Weapon" :!type "Name") _returnvalue_2)
  (`self.K2_AttachToComponent` _returnvalue_2 (`self.Mesh`) "WeaponSocketR" "SnapToTarget" "SnapToTarget" "SnapToTarget" true))

(event `Key|R`
  (params (Key :type "Key Structure"))
  (:`Pressed`
    (`GameplayStatics.OpenLevelBySoftObjectPtr` "/Game/Maps/VelkariiPlayground.VelkariiPlayground")))

(fn `UserConstructionScript`)