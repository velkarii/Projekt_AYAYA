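; Player Blueprint with a toggleable target lock on the Tab key.
; Tab alternates between a sphere trace along the camera's forward vector, storing the hit Pawn-type actor as HitTarget, and clearing that target.
; While HitTarget is valid, Tick sets the control rotation to face it, with pitch clamped to a limited range.
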(event `self.ReceiveTick`
  (params (DeltaSeconds :type "Float (single-precision)"))
  ; Set Target Lock Rotation
  (`self.Hit Target`
    (:`then`
      (`Controller.SetControlRotation` (`self.GetController`) (`KismetMathLibrary.MakeRotator` (.roll (`KismetMathLibrary.FindLookAtRotation` (`self.K2_GetActorLocation`) (`self.K2_GetActorLocation` (`self.Hit Target`)))) (`KismetMathLibrary.FClamp` (.pitch (`KismetMathLibrary.FindLookAtRotation` (`self.K2_GetActorLocation`) (`self.K2_GetActorLocation` (`self.Hit Target`)))) -20.0 45.0) (.yaw (`KismetMathLibrary.FindLookAtRotation` (`self.K2_GetActorLocation`) (`self.K2_GetActorLocation` (`self.Hit Target`)))))))
    (:`else`)))

(event `Key|Tab`
  (params (Key :type "Key Structure"))
  (bind _returnvalue (`self.K2_GetActorLocation`))
  ; Target Lock
  (:`Pressed`
    (`/Engine/EditorBlueprintResources/StandardMacros.FlipFlop`
      (:`A`
        (bind (_outhit _returnvalue_2) (`KismetSystemLibrary.SphereTraceSingleForObjects` :`Start` _returnvalue :`End` (+ _returnvalue (* (`KismetMathLibrary.GetForwardVector` (`SceneComponent.K2_GetComponentRotation` (`self.Camera`))) 500.0)) :`Radius` 125.0 :`ObjectTypes` (`|MakeArray` "ObjectTypeQuery3" :!type "EObjectTypeQuery Enum") :`DrawDebugType` "ForDuration"))
        (if _returnvalue_2
          (set `self.Hit Target` (`.HitActor` (`GameplayStatics.BreakHitResult` _outhit)))))
      (:`B`
        (set `self.Hit Target` null)))))

(fn `UserConstructionScript`)